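; BPC_InteractionComponent is an interaction component that tracks whether something is interactable and whether an interaction is active.
; Enable and disable events set the Interactable flag and broadcast the change through OnToggleInteractability.
; StartInteraction fires OnInteract with the interacting actor only when interactable and not already activated, then marks it activated.
; EndInteracton fires OnInteract as off and clears the activated state without any checks.
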(event Custom|OnDisableInteractability
  (Variables|Default|SetInteractable false)
  (Default|CallOnToggleInteractability false))

(event Custom|OnEnableInteractability
  (Variables|Default|SetInteractable true)
  (Default|CallOnToggleInteractability true))

(event Custom|EndInteracton
  (Default|CallOnInteract false)
  (Variables|Default|SetActivated false))

(event Custom|StartInteraction
  (params (InteractingActor :type Actor%20Object%20Reference))
  (if (and (Variables|Default|GetInteractable) (not (Variables|Default|GetActivated)))
    (Default|CallOnInteract true InteractingActor)
    (Variables|Default|SetActivated true)))