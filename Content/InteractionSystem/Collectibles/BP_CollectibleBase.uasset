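; BP_CollectibleBase is the base actor for world items that a character picks up by interacting with them.
; Interact casts the character's controller to BP_PlayerController, adds one ItemData to its inventory, and destroys the actor only if the add succeeds.
; GetActionText and GetName supply the "pick up" verb and the item's name from ItemData.
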(event EventInteract
  (params (Interacting%20Character :type Character%20Object%20Reference))
  (bind _asbp_player_controller (Utilities|Casting|CastToBP_PlayerController (Pawn|GetController Interacting%20Character)))
  (bind _returnvalue (Class|XPlayerController|AddInventoryItem _asbp_player_controller (Variables|Default|GetItem%20Data) 1))
  (if _returnvalue
    (Actor|DestroyActor)))

(fn ConstructionScript)

(fn GetActionText
  (return "pick up"))

(fn GetName
  (return (Variables|/Script/Explore.XItem|GetName (Variables|Default|GetItem%20Data))))