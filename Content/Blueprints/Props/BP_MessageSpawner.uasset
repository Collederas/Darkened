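; BP_MessageSpawner is a trigger prop that shows the WB_FinalText message when the first-person player walks into its box.
; On BeginPlay it creates the widget up front and keeps a reference to it.
; On overlap it stops the character's movement, adds the widget to the viewport, switches input to UI-only and pauses the game.
; The end-overlap handler only casts and does nothing further.
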(event OnComponentBeginOverlap(Box)
  (params (OverlappedComponent :type Primitive%20Component%20Object%20Reference) (OtherActor :type Actor%20Object%20Reference) (OtherComp :type Primitive%20Component%20Object%20Reference) (OtherBodyIndex :type Integer) (bFromSweep :type Boolean) (SweepResult :type Hit%20Result%20Structure%20%28by%20ref%29))
  (bind _widget (Variables|Default|GetWidget))
  (bind _asfirst_person_character (Utilities|Casting|CastToFirstPersonCharacter OtherActor))
  (Components|Movement|StopMovementImmediately (Pawn|GetMovementComponent _asfirst_person_character))
  (UserInterface|Viewport|AddtoViewport _widget 0)
  (Input|SetInputModeUIOnly (Game|GetPlayerController 0) _widget "DoNotLock")
  (Game|SetGamePaused true))

(event OnComponentEndOverlap(Box)
  (params (OverlappedComponent :type Primitive%20Component%20Object%20Reference) (OtherActor :type Actor%20Object%20Reference) (OtherComp :type Primitive%20Component%20Object%20Reference) (OtherBodyIndex :type Integer))
  (Utilities|Casting|CastToFirstPersonCharacter OtherActor))

(event EventBeginPlay
  (bind _returnvalue (UserInterface|CreateWidget "/Game/UI/WB_FinalText.WB_FinalText_C" (Game|GetPlayerController 0)))
  (Variables|Default|SetWidget _returnvalue))

(fn ConstructionScript)