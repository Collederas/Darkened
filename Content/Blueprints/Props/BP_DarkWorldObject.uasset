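; BP_DarkWorldObject is a prop that appears or disappears when dark mode is toggled.
; The DarkWorldAppear flag chooses whether the object is present in dark mode or only outside it.
; ToggleDarkMode switches the static mesh's visibility and swaps its collision profile between BlockAllDynamic and IgnoreOnlyPawn, so hidden objects let pawns through.
; The Freeze event sets a flag that makes the object ignore toggles, holding its current state.
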(event EventFreeze
  (params (On :type Boolean))
  (Variables|Default|SetFrozen On))

(event EventToggleDarkMode
  (params (On :type Boolean))
  (if (not (Variables|Default|GetFrozen))
    (if (Variables|Default|GetDarkWorldAppear)
      (if On
        (Rendering|SetVisibility (Variables|Default|GetStaticMesh) true false)
        (Collision|SetCollisionProfileName (Variables|Default|GetStaticMesh) "BlockAllDynamic" true :!class /Script/Engine.PrimitiveComponent)
        (else
          (Rendering|SetVisibility (Variables|Default|GetStaticMesh) false false)
          (Collision|SetCollisionProfileName (Variables|Default|GetStaticMesh) "IgnoreOnlyPawn" true :!class /Script/Engine.PrimitiveComponent)))
      (elif On
        (Rendering|SetVisibility (Variables|Default|GetStaticMesh) false false)
        (Collision|SetCollisionProfileName (Variables|Default|GetStaticMesh) "IgnoreOnlyPawn" true :!class /Script/Engine.PrimitiveComponent)
        (else
          (Rendering|SetVisibility (Variables|Default|GetStaticMesh) true false)
          (Collision|SetCollisionProfileName (Variables|Default|GetStaticMesh) "BlockAllDynamic" true :!class /Script/Engine.PrimitiveComponent))))))

(fn ConstructionScript)