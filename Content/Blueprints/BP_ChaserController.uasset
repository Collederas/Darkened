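; AI controller for the Chaser enemy that runs Chaser_BT on possession and tracks the player through AI perception.
; Sensing a Player-tagged actor clears the loss timer and sets HasLineOfSight and Target in the Blackboard.
; Any other perception update starts a delay timer that clears both keys on expiry.
; A helper, uncalled here, adjusts post-process vignette and grain from distance versus range.
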(event OnTargetPerceptionUpdated(AIPerception)
  (params (Actor :type Actor%20Object%20Reference) (Stimulus :type AI%20Stimulus%20Structure))
  (bind _blackboard (Variables|Default|GetBlackboard))
  (if (and (Actor|ActorHasTag Actor "Player") (.bSuccessfullySensed (Utilities|Struct|BreakAIStimulus Stimulus))) ; Floof
    (Utilities|Time|ClearandInvalidateTimerbyHandle (Variables|Default|GetEnemySightTimer))
    (AI|Components|Blackboard|SetValueasBool _blackboard (Variables|Default|GetHasLineOfSight) true)
    (AI|Components|Blackboard|SetValueasObject _blackboard (Variables|Default|GetTarget) Actor)
    (else
      (bind _returnvalue (Utilities|Time|SetTimerbyEvent (delegate Custom|StartEnemyTimer) (Variables|Default|GetLineOfSightTimer)))
      (Variables|Default|SetEnemySightTimer _returnvalue))))

(event Custom|StartEnemyTimer
  (bind _blackboard (Variables|Default|GetBlackboard))
  (AI|Components|Blackboard|SetValueasBool _blackboard (Variables|Default|GetHasLineOfSight) false)
  (AI|Components|Blackboard|SetValueasObject _blackboard (Variables|Default|GetTarget) 0))

(event EventPossess
  (params (PossessedPawn :type Pawn%20Object%20Reference))
  (Variables|Default|SetPossessed%20Pawn PossessedPawn)
  (AI|RunBehaviorTree "/Game/AI/Chaser_BT.Chaser_BT"))

(fn ConstructionScript)

(fn ChangePostProcessEffect
  (params (Post%20Process%20Object :type Post%20Process%20Component%20Object%20Reference) (Distance :type Float%20%28single-precision%29%20%28by%20ref%29) (Range :type Float%20%28single-precision%29%20%28by%20ref%29))
  (bind _returnvalue (- Range Distance))
  (bind _returnvalue_2 (/ _returnvalue Range))
  (if (>= Range Distance)
    (bind _structout (Utilities|Struct|SetmembersinPostProcessSettings (Variables|/Script/Engine.PostProcessComponent|GetSettings Post%20Process%20Object) 0.0))
    (else
      (Utilities|Struct|SetmembersinPostProcessSettings (Variables|/Script/Engine.PostProcessComponent|GetSettings Post%20Process%20Object) _returnvalue_2 _returnvalue_2 _returnvalue_2)))
  (Variables|/Script/Engine.PostProcessComponent|SetSettings Post%20Process%20Object _structout)
  (return))

(fn ChangePostProcessEffect23)