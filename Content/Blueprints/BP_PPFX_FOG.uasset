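; BP_PPFX_FOG switches post-process visuals between a dark and a light mode.
; The ToggleDarkMode event passes its flag and the PostProcessing reference to ToggleDarkModeFX, which edits that object's post-process settings.
; Dark mode lowers overall gamma and sets an intensity value, while light mode uses neutral gamma; saturation is neutral in both.
; ToggleDarkModeFog is an uncalled stub that leaves the height fog unchanged.
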(event EventBeginPlay)

(event Collision|EventActorBeginOverlap
  (params (OtherActor :type Actor%20Object%20Reference)))

(event EventTick
  (params (DeltaSeconds :type Float%20%28single-precision%29)))

(event EventToggleDarkMode
  (params (On :type Boolean))
  (CallFunction|ToggleDarkModeFX On (Variables|Default|GetPost%20Processing)))

(fn ConstructionScript)

(fn ToggleDarkModeFX
  (params (isDark :type Boolean) (Post%20Processsing :type Post%20Process%20Component%20Object%20Reference))
  (if isDark
    (bind _structout (Utilities|Struct|SetmembersinPostProcessSettings (Variables|/Script/Engine.PostProcessComponent|GetSettings Post%20Processsing) (Math|Vector4|MakeVector4 1.0 1.0 1.0 1.0) (Math|Vector4|MakeVector4 1.0 1.0 1.0 0.4) 3.0))
    (else
      (Utilities|Struct|SetmembersinPostProcessSettings (Variables|/Script/Engine.PostProcessComponent|GetSettings Post%20Processsing) (Math|Vector4|MakeVector4 1.0 1.0 1.0 1.0) (Math|Vector4|MakeVector4 1.0 1.0 1.0 1.0))))
  (Variables|/Script/Engine.PostProcessComponent|SetSettings Post%20Processsing _structout)
  (return))

(fn ToggleDarkModeFog
  (params (isDark :type Boolean) (ExponentialHeightFog%20 :type Exponential%20Height%20Fog%20Object%20Reference))
  (if isDark
    _))