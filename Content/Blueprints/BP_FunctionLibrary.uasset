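; Blueprint function library for switching the game's dark world mode and finding the closest actor overlapping a target.
; ToggleDarkMode messages every BPI_Darken implementer, rotates the sun and has the game instance fade sound.
; SetDarkWorldObjectsVisibility shows or hides "Dark"-tagged actors and passes the state to chaser characters; its static mesh collision switch sits behind that chaser cast.
; GetClosestOverlappingActor compares squared distances.
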(fn GetClosestOverlappingActor
  (params (TargetActor :type Actor%20Object%20Reference))
  (bind _overlappingactors (Collision|GetOverlappingActors TargetActor "/Script/Engine.Actor" :!class /Script/Engine.Actor))
  (if (== (Utilities|Array|Length _overlappingactors) 1)
    (return (Utilities|Array|Get(acopy) _overlappingactors))
    (else
      (for (_array_element _array_index) _overlappingactors
        (if (== _array_index 0)
          (bind _output_get (LocalVariables|SetMinDistanceSquared (Transformation|GetSquaredDistanceTo _array_element TargetActor)))
          (Math|Float|IncrementFloat _output_get
            (:%20%20
              _)))
        (Math|Float|CompareFloat (Transformation|GetSquaredDistanceTo _array_element TargetActor) (LocalVariables|GetMinDistanceSquared)
          (:<
            (LocalVariables|SetMinDistanceSquared (Transformation|GetSquaredDistanceTo _array_element TargetActor))
            (LocalVariables|SetClosestActor _array_element))))
      (return (LocalVariables|GetClosestActor)))))

(fn SetDarkWorldObjectsVisibility
  (params (Visible :type Boolean))
  (bind _outactors (Actor|GetAllActorswithTag 0 "Dark"))
  (for _array_element _outactors
    (Rendering|SetActorHiddenInGame _array_element (not Visible))
    (bind _asbp_chaser_character (Utilities|Casting|CastToBP_ChaserCharacter _array_element))
    (Utilities|IsValid _asbp_chaser_character
      (:Is%20Valid
        (Default|ToggleDarkMode _asbp_chaser_character Visible))
      (:Is%20Not%20Valid
        (Utilities|IsValid (Actor|GetComponentbyClass _array_element "/Script/Engine.StaticMeshComponent")
          (:Is%20Valid
            (if Visible
              (Collision|SetCollisionProfileName (Actor|GetComponentbyClass _array_element "/Script/Engine.StaticMeshComponent") "Pawn" true :!class /Script/Engine.PrimitiveComponent)
              (else
                (Collision|SetCollisionProfileName (Actor|GetComponentbyClass _array_element "/Script/Engine.StaticMeshComponent") "IgnoreOnlyPawn" true :!class /Script/Engine.PrimitiveComponent)))))))))

(fn ToggleDarkMode
  (params (Sun :type Directional%20Light%20Object%20Reference) (On :type Boolean) (GameInstance :type BP%20Game%20Instance%20Object%20Reference))
  (if On
    (bind _outactors (Actor|GetAllActorswithInterface 0 "/Game/Blueprints/BPI_Darken.BPI_Darken_C"))
    (for _array_element _outactors
      (Class|BPIDarken|ToggleDarkMode(Message) _array_element true))
    (Transformation|SetActorRotation Sun)
    (Default|FadetoSound GameInstance true)
    (else
      (bind _outactors_2 (Actor|GetAllActorswithInterface 0 "/Game/Blueprints/BPI_Darken.BPI_Darken_C"))
      (for _array_element_2 _outactors_2
        (Class|BPIDarken|ToggleDarkMode(Message) _array_element_2 false))
      (Transformation|SetActorRotation Sun "255.000000, 0, 0")
      (Default|FadetoSound GameInstance false))))