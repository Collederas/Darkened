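; BP_ChaserCharacter is an AI-driven chaser pawn with adjustable walk speed and a dark mode that controls its collision.
; On BeginPlay it caches its BP_ChaserController.
; UpdateSpeed sets the movement component's max walk speed.
; ToggleDarkMode swaps capsule and mesh collision profiles, restoring standard pawn collision when on, and ignoring pawns with mesh collision disabled when off.
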(event Custom|UpdateSpeed
  (params (NewSpeed :type Float%20%28single-precision%29))
  (Variables|/Script/Engine.CharacterMovementComponent|SetMaxWalkSpeed (Variables|Character|GetCharacterMovement) NewSpeed))

(event Custom|ToggleDarkMode
  (params (On :type Boolean))
  (bind _mesh (Variables|Character|GetMesh))
  (if On
    (Collision|SetCollisionProfileName (Variables|Collision|GetCapsuleComponent) "Pawn" true :!class /Script/Engine.PrimitiveComponent)
    (Collision|SetCollisionProfileName _mesh "CharacterMesh" true :!class /Script/Engine.PrimitiveComponent)
    (else
      (Collision|SetCollisionProfileName (Variables|Collision|GetCapsuleComponent) "IgnoreOnlyPawn" true :!class /Script/Engine.PrimitiveComponent)
      (Collision|SetCollisionProfileName _mesh "NoCollision" true :!class /Script/Engine.PrimitiveComponent))))

(event EventBeginPlay
  (bind _asbp_chaser_controller (Utilities|Casting|CastToBP_ChaserController (AI|GetAIController self)))
  (Variables|Default|SetChaserController _asbp_chaser_controller))

(fn ConstructionScript)